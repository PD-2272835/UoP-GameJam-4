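; BP_Mineral is a collectible mineral in the oxygen system that the player picks up by interacting with it.
; BeginPlay caches the third-person character, and OnInteract increments the MineralCount on that character's inventory component.
; It then finds every BP_UpgradeStation to refresh its requirements display, calling DestroyActor inside that loop, so the mineral only destroys itself if a station exists.
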(event `self.ReceiveBeginPlay`
  ;[0.1002 0.2859 0.2917] store reference to player to prevent multiple casts (expensive)
  (bind _asbp_third_person_character (cast `/Game/ThirdPerson/Blueprints/BP_ThirdPersonCharacter` (`GameplayStatics.GetPlayerPawn` 0)))
  (set `self.playerRef` _asbp_third_person_character))

(event `/Game/OxygenSystem/BPI_Interaction.OnInteract`
  (params (NewParam :type "/Game/OxygenSystem/BP_Interactable Object Reference"))
  (`/Engine/EditorBlueprintResources/StandardMacros.IncrementInt` (`/Game/OxygenSystem/CBP_PlayerInventory.mineralCount` (`/Game/ThirdPerson/Blueprints/BP_ThirdPersonCharacter.CBP_PlayerInventory` (`self.playerRef`))) ; give the player a mineral
    (:`  `
      ;[0.05502 0.2604 0.06765] shitty hack fix to update the display on each upgrade station from the mineral
      (bind _outactors (`GameplayStatics.GetAllActorsOfClass` "/Game/OxygenSystem/BP_UpgradeStation.BP_UpgradeStation_C"))
      (for _array_element _outactors
        (`/Game/OxygenSystem/BP_UpgradeStation.UpdateRequirementsDisplay` _array_element)
        (`self.K2_DestroyActor`)))))

(fn `UserConstructionScript`)