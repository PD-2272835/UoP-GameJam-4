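; BP_Base is an interactable base whose door teleports the player between inside and outside as part of the oxygen system.
; BeginPlay caches the player character's oxygen component to avoid repeated casts.
; OnInteract reads its IsOutside flag to call IngressPlayer or EgressPlayer, which teleport the pawn to the matching scene point.
; The flag flips only when the teleport succeeds; failures print a message.
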(event `self.ReceiveBeginPlay`
  ;[0.3938 0.1306 0.4479] store reference to player preventing multiple casts each time we need a value
  (bind _asbp_third_person_character (cast `/Game/ThirdPerson/Blueprints/BP_ThirdPersonCharacter` (`GameplayStatics.GetPlayerPawn` 0)))
  (set `self.OxygenSysRef` (`/Game/ThirdPerson/Blueprints/BP_ThirdPersonCharacter.CBP_OxygenSystem` _asbp_third_person_character)))

(event `/Game/OxygenSystem/BPI_Interaction.OnInteract`
  (params (NewParam :type "/Game/OxygenSystem/BP_Interactable Object Reference"))
  ;[0.1555 0.2148 0.4427] determine whether the player should enter or exit the base upon interacting with the door, based on the isOutside flag
  (if (`/Game/OxygenSystem/CBP_OxygenSystem.isOutside` (`self.OxygenSysRef`))
    (`self.IngressPlayer`)
    (else
      (`self.EgressPlayer`))))

(fn `EgressPlayer`
  (bind _egresspoint (`self.EgressPoint`))
  (bind _returnvalue (`self.K2_TeleportTo` (`GameplayStatics.GetPlayerPawn` 0) (`SceneComponent.K2_GetComponentLocation` _egresspoint) (`SceneComponent.K2_GetComponentRotation` _egresspoint)))
  (if _returnvalue
    (set `/Game/OxygenSystem/CBP_OxygenSystem.isOutside` true (`self.OxygenSysRef`))
    (else
      (`KismetSystemLibrary.PrintString` "Unable to exit base"))))

(fn `IngressPlayer`
  (bind _ingresspoint (`self.IngressPoint`))
  (bind _returnvalue (`self.K2_TeleportTo` (`GameplayStatics.GetPlayerPawn` 0) (`SceneComponent.K2_GetComponentLocation` _ingresspoint) (`SceneComponent.K2_GetComponentRotation` _ingresspoint)))
  (if _returnvalue
    (set `/Game/OxygenSystem/CBP_OxygenSystem.isOutside` false (`self.OxygenSysRef`))
    (else
      (`KismetSystemLibrary.PrintString` "Unable to enter base"))))

(fn `UserConstructionScript`)