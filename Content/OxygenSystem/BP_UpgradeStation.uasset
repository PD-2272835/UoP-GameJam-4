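; BP_UpgradeStation is an interactable station where the player spends minerals to upgrade their oxygen tank.
; On BeginPlay it caches the player character and its inventory component, which holds the mineral count, upgrade level and per-level cost and increment arrays.
; Interacting deducts the current cost, raises the level, passes the new level's increment to the oxygen system and refreshes the minerals/cost text, or prints a message when minerals fall short.
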(event `self.ReceiveBeginPlay`
  ;[0.1826 0.2969 0.1158] store reference to prevent multiple casts (expensive)
  (bind _asbp_third_person_character (cast `/Game/ThirdPerson/Blueprints/BP_ThirdPersonCharacter` (`GameplayStatics.GetPlayerPawn` 0)))
  (bind _output_get (set `self.playerRef` _asbp_third_person_character))
  (set `self.inventoryRef` (`/Game/ThirdPerson/Blueprints/BP_ThirdPersonCharacter.CBP_PlayerInventory` _output_get))
  (`self.UpdateRequirementsDisplay`))

(event `/Game/OxygenSystem/BPI_Interaction.OnInteract`
  (params (NewParam :type "/Game/OxygenSystem/BP_Interactable Object Reference"))
  (bind _inventoryref (`self.inventoryRef`))
  (bind _inventoryref_2 (`self.inventoryRef`))
  (bind _output (`|GetArrayItem` (`/Game/OxygenSystem/CBP_PlayerInventory.upgradeRequirements` _inventoryref_2) (`/Game/OxygenSystem/CBP_PlayerInventory.upgradeLevel` _inventoryref_2)))
  (if (>= (`/Game/OxygenSystem/CBP_PlayerInventory.mineralCount` _inventoryref_2) _output)
    (set `/Game/OxygenSystem/CBP_PlayerInventory.mineralCount` (- (`/Game/OxygenSystem/CBP_PlayerInventory.mineralCount` _inventoryref_2) _output) _inventoryref_2)
    (`/Engine/EditorBlueprintResources/StandardMacros.IncrementInt` (`/Game/OxygenSystem/CBP_PlayerInventory.upgradeLevel` _inventoryref)
      (:`  `
        (`/Game/OxygenSystem/CBP_OxygenSystem.UpgradeOxygen` (`/Game/ThirdPerson/Blueprints/BP_ThirdPersonCharacter.CBP_OxygenSystem` (`self.playerRef`)) (`|GetArrayItem` (`/Game/OxygenSystem/CBP_PlayerInventory.upgradeIncrements` _inventoryref) (`/Game/OxygenSystem/CBP_PlayerInventory.upgradeLevel` _inventoryref)))
        (`self.UpdateRequirementsDisplay`)))
    (else
      (`KismetSystemLibrary.PrintString` "not enough minerals"))))

(fn `UpdateRequirementsDisplay`
  (bind _inventoryref (`self.inventoryRef`))
  (`TextRenderComponent.K2_SetText` (`self.nextUpgradeReqDisplay`) (`KismetTextLibrary.Conv_StringToText` (`KismetStringLibrary.Concat_StrStr` (`KismetStringLibrary.Conv_IntToString` (`/Game/OxygenSystem/CBP_PlayerInventory.mineralCount` _inventoryref)) "/" (`KismetStringLibrary.Conv_IntToString` (`|GetArrayItem` (`/Game/OxygenSystem/CBP_PlayerInventory.upgradeRequirements` _inventoryref) (`/Game/OxygenSystem/CBP_PlayerInventory.upgradeLevel` _inventoryref)))))))

(fn `UserConstructionScript`)