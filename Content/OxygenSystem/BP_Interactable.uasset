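; BP_Interactable is a reusable interaction point that other actors attach as a child, with a configurable radius set in the construction script.
; Overlapping its sphere shows a prompt widget and registers it as the player's CurrentInteractable; ending overlap hides the prompt and clears only its own reference.
; OnInteract forwards to the parent actor's OnInteract message, passing itself so one parent can distinguish multiple points.
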(event `self.ReceiveBeginPlay`
  ;[0.1002 0.2859 0.2917] store reference to player to prevent multiple casts
  (bind _asbp_third_person_character (cast `/Game/ThirdPerson/Blueprints/BP_ThirdPersonCharacter` (`GameplayStatics.GetPlayerPawn` 0)))
  (set `self.playerRef` _asbp_third_person_character))

(event `self.InteractionRange.OnComponentBeginOverlap`
  (params (OverlappedComponent :type "PrimitiveComponent Object Reference") (OtherActor :type "Actor Object Reference") (OtherComp :type "PrimitiveComponent Object Reference") (OtherBodyIndex :type Integer) (bFromSweep :type Boolean) (SweepResult :type "HitResult Structure (by ref)"))
  ;[0.5833 0.3801 0.316] toggle interaction prompt depending on if the player is within interaction range or not
  (`SceneComponent.SetVisibility` (`self.Widget`) true false)
  ;[0.3263 0.5737 0.6458] ensure the player has a reference to this interaction point so that onInteract can be called from player input
  (set `/Game/ThirdPerson/Blueprints/BP_ThirdPersonCharacter.currentInteractable` self (`self.playerRef`)))

(event `self.InteractionRange.OnComponentEndOverlap`
  (params (OverlappedComponent :type "PrimitiveComponent Object Reference") (OtherActor :type "Actor Object Reference") (OtherComp :type "PrimitiveComponent Object Reference") (OtherBodyIndex :type Integer))
  ;[0.5833 0.3801 0.316] toggle interaction prompt depending on if the player is within interaction range or not
  (`SceneComponent.SetVisibility` (`self.Widget`) false false)
  ;[0.3263 0.5737 0.6458] ensure the player has a reference to this interaction point so that onInteract can be called from player input
  (if (== (`/Game/ThirdPerson/Blueprints/BP_ThirdPersonCharacter.currentInteractable` (`self.playerRef`)) self)
    (set `/Game/ThirdPerson/Blueprints/BP_ThirdPersonCharacter.currentInteractable` null (`self.playerRef`))))

(event `/Game/OxygenSystem/BPI_Interaction.OnInteract`
  (params (NewParam :type "/Game/OxygenSystem/BP_Interactable Object Reference"))
  ;[0.4705 0.2622 1] If this interaction point is interacted with, call oninteract on the parent object and identify this point so that multiple interactions on the same parent can do different things
  (message `/Game/OxygenSystem/BPI_Interaction.OnInteract` (`self.GetParentActor`) self))

(fn `UserConstructionScript`
  ;[0.3073 0.1008 0.1839] allow interaction distance to be changed when attached to another object
  (`SphereComponent.SetSphereRadius` (`self.InteractionRange`) (`self.interactionDistance`) true))